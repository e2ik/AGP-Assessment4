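; Player melee character Blueprint that handles the visual side of sword combat: slashes, sword display and a red flash.
; Local control selects first-person arms or the full-body Manny for mesh visibility, sword start/end points, montages and sword visibility.
; SwordSlashGraphical cycles a three-slash combo through CurrentSlash, which updates on montage start and Notify Begin.
; DisplayRedFlash blinks an overlay material on the Manny mesh three times using delays.
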(event EventBeginPlay
  (if (Pawn|IsLocallyControlled)
    (Variables|Default|SetSwordStartPosition (Variables|Default|GetSwordStart1))
    (Variables|Default|SetSwordEndPosition (Variables|Default|GetSwordEnd1))
    (Rendering|SetVisibility (Variables|Character|GetMesh) true false)
    (Rendering|SetVisibility (Variables|Default|GetSKM_Manny) false true)
    (else
      (Variables|Default|SetSwordStartPosition (Variables|Default|GetSwordStart))
      (Variables|Default|SetSwordEndPosition (Variables|Default|GetSwordEnd))
      (Rendering|SetVisibility (Variables|Character|GetMesh) false false)
      (Rendering|SetVisibility (Variables|Default|GetSKM_Manny) true true))))

(event Collision|EventActorBeginOverlap
  (params (OtherActor :type Actor%20Object%20Reference)))

(event EventTick
  (params (DeltaSeconds :type Float%20%28single-precision%29)))

(event EventSwordSlashGraphical
  (bind _skm_manny (Variables|Default|GetSKM_Manny))
  (if (Pawn|IsLocallyControlled)
    (switch int (Variables|Default|GetCurrentSlash)
      (:0
        (Animation|Montage|PlayMontage (Variables|Character|GetMesh) "/Game/Assets/KoreanTraditionalMartialArts/RetargetedArmAnims/Arms_Slash_1.Arms_Slash_1"
          (:then
            _)
          (:OnNotifyBegin
            _))
        (Variables|Default|SetCurrentSlash (+ (Variables|Default|GetCurrentSlash) 1) :!label _label))
      (:1
        (Animation|Montage|PlayMontage (Variables|Character|GetMesh) "/Game/Assets/KoreanTraditionalMartialArts/RetargetedArmAnims/Arms_Slash_2.Arms_Slash_2"
          (:then
            (goto _label))
          (:OnNotifyBegin
            (goto _label))))
      (:2
        (Animation|Montage|PlayMontage (Variables|Character|GetMesh) "/Game/Assets/KoreanTraditionalMartialArts/RetargetedArmAnims/Arms_Slash_3.Arms_Slash_3"
          (:then
            _)
          (:OnNotifyBegin
            _))
        (Variables|Default|SetCurrentSlash 0 :!label _label_2)))
    (else
      (switch int (Variables|Default|GetCurrentSlash)
        (:0
          (Animation|Montage|PlayMontage _skm_manny "/Game/Assets/KoreanTraditionalMartialArts/RetargetedFullBodyAnims/FullBody_Slash_1.FullBody_Slash_1"
            (:then
              (goto _label))
            (:OnNotifyBegin
              (goto _label))))
        (:1
          (Animation|Montage|PlayMontage _skm_manny "/Game/Assets/KoreanTraditionalMartialArts/RetargetedFullBodyAnims/FullBody_Slash2.FullBody_Slash2"
            (:then
              (goto _label))
            (:OnNotifyBegin
              (goto _label))))
        (:2
          (Animation|Montage|PlayMontage _skm_manny "/Game/Assets/KoreanTraditionalMartialArts/RetargetedFullBodyAnims/FullBody_Slash3.FullBody_Slash3"
            (:then
              (goto _label_2))
            (:OnNotifyBegin
              (goto _label_2))))))))

(event EventEquipSwordGraphical
  (params (bEquipWeapon :type Boolean) (SwordStats :type Sword%20Stats%20Structure))
  (if (Pawn|IsLocallyControlled)
    (Rendering|SetVisibility (Variables|Default|GetArmsSword) bEquipWeapon false)
    (else
      (Rendering|SetVisibility (Variables|Default|GetFullBodySword) bEquipWeapon false))))

(event EventChooseCharacterMesh
  (if (Pawn|IsLocallyControlled)
    (Variables|Default|SetSwordStartPosition (Variables|Default|GetSwordStart1))
    (Variables|Default|SetSwordEndPosition (Variables|Default|GetSwordEnd1))
    (Rendering|SetVisibility (Variables|Character|GetMesh) true false)
    (Rendering|SetVisibility (Variables|Default|GetSKM_Manny) false true)
    (else
      (Variables|Default|SetSwordStartPosition (Variables|Default|GetSwordStart))
      (Variables|Default|SetSwordEndPosition (Variables|Default|GetSwordEnd))
      (Rendering|SetVisibility (Variables|Character|GetMesh) false false)
      (Rendering|SetVisibility (Variables|Default|GetSKM_Manny) true true))))

(event EventDisplayRedFlash
  (bind _skm_manny (Variables|Default|GetSKM_Manny))
  (Rendering|Material|SetOverlayMaterial _skm_manny "/Engine/MapTemplates/Materials/BasicAsset01.BasicAsset01" :!class /Script/Engine.MeshComponent)
  (Utilities|FlowControl|Delay 0.1)
  (Rendering|Material|SetOverlayMaterial _skm_manny 0 :!class /Script/Engine.MeshComponent)
  (Utilities|FlowControl|Delay 0.1)
  (Rendering|Material|SetOverlayMaterial _skm_manny "/Engine/MapTemplates/Materials/BasicAsset01.BasicAsset01" :!class /Script/Engine.MeshComponent)
  (Utilities|FlowControl|Delay 0.1)
  (Rendering|Material|SetOverlayMaterial _skm_manny 0 :!class /Script/Engine.MeshComponent)
  (Utilities|FlowControl|Delay 0.1)
  (Rendering|Material|SetOverlayMaterial _skm_manny "/Engine/MapTemplates/Materials/BasicAsset01.BasicAsset01" :!class /Script/Engine.MeshComponent)
  (Utilities|FlowControl|Delay 0.1)
  (Rendering|Material|SetOverlayMaterial _skm_manny 0 :!class /Script/Engine.MeshComponent))

(fn ConstructionScript)